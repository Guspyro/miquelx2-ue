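; AI controller for NPC characters that runs the BT_NPC behavior tree on possession and on begin play.
; Perception updates write whether the stimulus was sensed into the CanSeePlayer blackboard key.
; A kill event sets the IsRagdoll key to exit the tree, then tells the controlled Character_NPC to ragdoll.
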(event `self.ReceivePossess`
  (params (PossessedPawn :type "Pawn Object Reference"))
  ;[1 1 1] On start or posses, run BT
  (`self.RunBehaviorTree` "/Game/Blueprints/AI/BT_NPC.BT_NPC" :!label _label))

(event `self.ReceiveBeginPlay`
  ;[1 1 1] On start or posses, run BT
  (goto _label))

(event `EventKill`
  ;[1 1 1] Exit tree
  (`BlackboardComponent.SetValueAsBool` (`AIBlueprintHelperLibrary.GetBlackboard` self) "IsRagdoll" true)
  ;[1 1 1] Do ragdoll
  (bind _ascharacter_npc (cast `/Game/Blueprints/AI/Character_NPC` (`self.K2_GetPawn` self)))
  (`/Game/Blueprints/AI/Character_NPC.DoRagdoll` _ascharacter_npc))

(event `self.AIPerception.OnTargetPerceptionUpdated`
  (params (Actor :type "Actor Object Reference") (Stimulus :type "AIStimulus Structure"))
  (`BlackboardComponent.SetValueAsBool` (`AIBlueprintHelperLibrary.GetBlackboard` self) "CanSeePlayer" (`.bSuccessfullySensed` (break `AIStimulus` Stimulus))))

(fn `UserConstructionScript`)