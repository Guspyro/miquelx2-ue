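; MySavegame is a savegame Blueprint that records the player's transform, items and NPC transforms.
; StartSave clears the item and NPC collections, leaving the player transform untouched.
; SavePlayer stores the passed transform, and SaveItem adds items without duplicates.
; SaveNPC maps each NPC reference to its current actor transform; the file has no load or disk-write logic.
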(fn `SaveItem`
  (params (NewItem :type "/Game/Blueprints/Interactables/Items/Item Object Reference (by ref)"))
  (`KismetArrayLibrary.Array_AddUnique` (`self.existingItems`) NewItem))

(fn `SaveNPC`
  (params (NPC :type "/Game/Blueprints/AI/Character_NPC Object Reference (by ref)"))
  (`BlueprintMapLibrary.Map_Add` (`self.existingNPC`) NPC (`Actor.GetTransform` NPC)))

(fn `SavePlayer`
  (params (PlayerTransform :type "Transform Structure"))
  (set `self.PlayerTransform` PlayerTransform))

(fn `StartSave`
  (`KismetArrayLibrary.Array_Clear` (`self.existingItems`))
  (`BlueprintMapLibrary.Map_Clear` (`self.existingNPC`)))