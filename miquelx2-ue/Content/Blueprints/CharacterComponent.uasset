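; Character component that handles death and respawn for its owning actor.
; On BeginPlay it stores the owner's transform as the respawn point.
; Die creates the game-over widget if none is valid, reuses it otherwise, and adds it to the viewport.
; Respawn removes that widget and moves the owner back to the stored transform without sweep or teleport physics.
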(event `self.ReceiveBeginPlay`
  ;[1 1 1] Begin
  (set `self.respawnTransform` (`Actor.GetTransform` (`self.GetOwner`))))

(fn `Die`
  (`/Engine/EditorBlueprintResources/StandardMacros.IsValid` (`self.GameOverUI`)
    (:`Is Valid`
      _)
    (:`Is Not Valid`
      (bind _returnvalue (`|CreateWidget` "/Game/UI/GameOverUI.GameOverUI_C"))
      (set `self.GameOverUI` _returnvalue)))
  (`UserWidget.AddToViewport` (`self.GameOverUI`) 0))

(fn `Respawn`
  (`Widget.RemoveFromParent` (`self.GameOverUI`))
  (`Actor.K2_SetActorTransform` (`self.GetOwner`) (`self.respawnTransform`) false false))