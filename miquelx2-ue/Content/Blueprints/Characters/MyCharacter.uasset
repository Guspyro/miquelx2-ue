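; Player character Blueprint that tracks coins and unique keys, with game-over, respawn and save/load of its transform.
; Overlaps call Interact and EndInteract on IInteractable actors, while the interact event presses the current Puzzle's button.
; Coin pickups trigger a HUD animation, and Confuse sets a timed flag.
; Die shows a lazily created game-over widget; Respawn removes it and restores the transform recorded at BeginPlay.
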(event `self.ReceiveBeginPlay`
  ;[1 1 1] Begin Play
  (set `self.respawnTransform` (`self.GetTransform`)))

(event `self.ReceiveActorBeginOverlap`
  (params (OtherActor :type "Actor Object Reference"))
  ;[1 1 1] Start/End interact
  (bind _asiinteractable (cast `/Game/Blueprints/Interactables/IInteractable` OtherActor))
  (`/Game/Blueprints/Interactables/IInteractable.Interact` _asiinteractable))

(event `self.ReceiveActorEndOverlap`
  (params (OtherActor :type "Actor Object Reference"))
  ;[1 1 1] Start/End interact
  (bind _asiinteractable (cast `/Game/Blueprints/Interactables/IInteractable` OtherActor))
  (`/Game/Blueprints/Interactables/IInteractable.EndInteract` _asiinteractable))

(event `EInteract`
  (bind _puzzle (`self.puzzle`))
  ;[1 1 1] E Pressed
  (`/Engine/EditorBlueprintResources/StandardMacros.IsValid` _puzzle
    (:`Is Valid`
      (`/Game/Blueprints/Interactables/Puzzle.ButtonPressed` _puzzle))))

(event `Confuse`
  ;[1 1 1] Confuse
  (set `self.confused` true)
  (`KismetSystemLibrary.Delay` (`self.confusionDuration`))
  (set `self.confused` false))

(event `/Game/Blueprints/Savegames/Storable.Save`
  (params (MySavegame :type "/Game/Blueprints/Savegames/MySavegame Object Reference"))
  (`/Game/Blueprints/Savegames/MySavegame.SavePlayer` MySavegame (`self.GetTransform`)))

(event `/Game/Blueprints/Savegames/Storable.Load`
  (params (MySavegame :type "/Game/Blueprints/Savegames/MySavegame Object Reference"))
  (`self.K2_SetActorTransform` (`/Game/Blueprints/Savegames/MySavegame.PlayerTransform` MySavegame)))

(fn `AddCoin`
  (bind _result (`/Engine/EditorBlueprintResources/StandardMacros.IncrementInt` (`self.Coins`))
    (:`  `
      (set `self.Coins` _result)
      (bind _asmy_hud (cast `/Game/Blueprints/Controllers/MyHUD` (`PlayerController.GetHUD` (`GameplayStatics.GetPlayerController` 0))))
      (`/Game/Blueprints/Controllers/MyHUD.PlayCoinAnimation` _asmy_hud))))

(fn `AddKey`
  (params (keyId :type String))
  (`KismetArrayLibrary.Array_AddUnique` (`self.keys`) keyId))

(fn `Die`
  (`self.GameOverUI`
    (:`then`
      _)
    (:`else`
      (bind _returnvalue (`|CreateWidget` "/Game/UI/GameOverUI.GameOverUI_C"))
      (set `self.GameOverUI` _returnvalue)))
  (`UserWidget.AddToViewport` (`self.GameOverUI`) 0))

(fn `Respawn`
  (`Widget.RemoveFromParent` (`self.GameOverUI`))
  (`self.K2_SetActorTransform` (`self.respawnTransform`)))

(fn `UserConstructionScript`)