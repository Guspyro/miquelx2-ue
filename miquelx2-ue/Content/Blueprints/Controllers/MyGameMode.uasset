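; Game mode that manages per-level save and load, plus a pause helper.
; On BeginPlay it uses the level name as the save slot, turns off the player controller's UI mode, then loads the existing save or creates a new MySavegame object.
; Saving and loading pass that object to every actor implementing the Storable interface via SaveMessage and LoadMessage, so each handles its own state.
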(event `self.ReceiveBeginPlay`
  (bind _returnvalue (`GameplayStatics.GetCurrentLevelName` true))
  (set `self.SaveGameSlot` _returnvalue)
  (`/Game/Blueprints/Controllers/MyPlayerController.disableUIMode` (`/Game/Libraries/MyCastLibrary.GetPlayerControllerAsMyPlayerController`))
  (bind _returnvalue_2 (`GameplayStatics.DoesSaveGameExist` (`self.SaveGameSlot`)))
  (if _returnvalue_2
    (`self.LoadGame`)
    (else
      (bind _returnvalue_3 (`GameplayStatics.CreateSaveGameObject` "/Game/Blueprints/Savegames/MySavegame.MySavegame_C"))
      (set `self.MySaveGame` _returnvalue_3))))

(fn `LoadGame`
  (bind _returnvalue (`GameplayStatics.LoadGameFromSlot` (`self.SaveGameSlot`)))
  (bind _asmy_savegame (cast `/Game/Blueprints/Savegames/MySavegame` _returnvalue))
  (set `self.MySaveGame` _asmy_savegame)
  (bind _outactors (`GameplayStatics.GetAllActorsWithInterface` "/Game/Blueprints/Savegames/Storable.Storable_C"))
  (for _array_element _outactors
    (message `/Game/Blueprints/Savegames/Storable.Load` _array_element (`self.MySaveGame`)))
  (`KismetSystemLibrary.PrintString` "Game Loaded" true true (struct :`G` 1.0 :`B` 0.15713 :`A` 1.0)))

(fn `PauseGame`
  (params (pause :type Boolean))
  (`GameplayStatics.SetGamePaused` pause))

(fn `SaveGame`
  (bind _mysavegame (`self.MySaveGame`))
  (bind _outactors (`GameplayStatics.GetAllActorsWithInterface` "/Game/Blueprints/Savegames/Storable.Storable_C"))
  (for _array_element _outactors
    (message `/Game/Blueprints/Savegames/Storable.Save` _array_element _mysavegame))
  (`GameplayStatics.SaveGameToSlot` _mysavegame (`self.SaveGameSlot`))
  (`KismetSystemLibrary.PrintString` "Game Saved" true true (struct :`R` 0.070746 :`G` 1.0 :`A` 1.0)))

(fn `UserConstructionScript`)