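; Elevator actor that moves continuously up and down along the Z axis.
; Each tick it offsets its location by Speed scaled to centimeters and adds the same step to CurrentHeight.
; When CurrentHeight reaches MaxHeight (also scaled to centimeters) or drops to zero or below, Speed flips sign to reverse direction.
; Movement is unswept, so it ignores blocking collision.
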(event `self.ReceiveTick`
  (params (DeltaSeconds :type "Float (single-precision)"))
  (bind _returnvalue (* DeltaSeconds (`self.speed`) 100.0))
  (`self.K2_SetActorLocation` (`KismetMathLibrary.MakeVector` (.x (`self.K2_GetActorLocation`)) (.y (`self.K2_GetActorLocation`)) (+ (.z (`self.K2_GetActorLocation`)) _returnvalue)))
  (bind _output_get (set `self.currentHeight` (+ _returnvalue (`self.currentHeight`))))
  (if (or (>= _output_get (* (`self.maxHeight`) 100.0)) (<= _output_get 0.0))
    (set `self.speed` (* (`self.speed`) -1.0))))

(fn `UserConstructionScript`)