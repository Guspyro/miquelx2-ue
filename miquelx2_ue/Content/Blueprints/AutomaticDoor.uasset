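; Automatic door actor that opens when a MyCharacter overlaps it and closes when that character leaves.
; BeginPlay stores the Door component's world location as the resting position.
; Overlap begin plays the Open timeline and overlap end reverses it, with each update setting the door to that position plus the Movement track's offset, without sweeping.
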(event `self.ReceiveBeginPlay`
  (set `self.InitialLocation` (`SceneComponent.K2_GetComponentLocation` (`self.Door`))))

(event `self.ReceiveActorBeginOverlap`
  (params (OtherActor :type "Actor Object Reference"))
  (cast `/Game/Blueprints/MyCharacter` OtherActor)
  (bind (_direction _movement) (`Timeline|Open` :!label _label)
    (:`Update`
      (`SceneComponent.K2_SetWorldLocation` (`self.Door`) (+ _movement (`self.InitialLocation`)) false false))))

(event `self.ReceiveActorEndOverlap`
  (params (OtherActor :type "Actor Object Reference"))
  (cast `/Game/Blueprints/MyCharacter` OtherActor)
  (goto _label :!via `Reverse`))

(fn `UserConstructionScript`)